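; BP_TrialsProximityObjective is a Trials objective that a player completes by overlapping the actor with their controlled pawn.
; On cosmetic-capable instances, the Icon starts hidden and each Tick shows it only while ObjectiveInfo reports the objective enabled for player controller 0.
; On the authority, an overlap by a pawn with a UTPlayerController calls CompleteObjective on ObjectiveInfo for that controller.
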(event `self.ReceiveBeginPlay`
  (`/Engine/EditorBlueprintResources/StandardMacros.Can Execute Cosmetic Events`
    (:`True`
      (`SceneComponent.SetVisibility` (`self.Icon`) false false))))

(event `self.ReceiveTick`
  (params (DeltaSeconds :type "Float (single-precision)"))
  (`/Engine/EditorBlueprintResources/StandardMacros.Can Execute Cosmetic Events`
    (:`True`
      (bind _asutplayer_controller (cast `UTPlayerController` (`GameplayStatics.GetPlayerController` 0)))
      (bind _returnvalue (`TrialsObjectiveInfo.IsEnabled` (`self.ObjectiveInfo`) _asutplayer_controller))
      (`SceneComponent.SetVisibility` (`self.Icon`) _returnvalue false))))

(event `self.ReceiveActorBeginOverlap`
  (params (OtherActor :type "Actor Object Reference"))
  (`/Engine/EditorBlueprintResources/ActorMacros.Switch Has Authority`
    (:`Authority`
      (bind _aspawn (cast `Pawn` OtherActor))
      (bind _asutplayer_controller (cast `UTPlayerController` (`Pawn.GetController` _aspawn)))
      (`TrialsObjectiveInfo.CompleteObjective` (`self.ObjectiveInfo`) _asutplayer_controller))))

(fn `UserConstructionScript`)