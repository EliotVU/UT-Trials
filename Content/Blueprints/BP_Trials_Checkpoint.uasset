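; Trials mode checkpoint actor that records itself as a player's checkpoint when their character touches it.
; On the authority, a collision overlap passes the actor to the character's TrialsPlayerController via SetCheckpoint.
; If the controller's CheckpointDest is then valid, it plays a teleport sound, spawns an attached particle effect and sends a localized message.
; The construction script sets the actor's rotation to the Arrow component's world rotation.
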(event `self.Collision.OnComponentBeginOverlap`
  (params (OverlappedComponent :type "PrimitiveComponent Object Reference") (OtherActor :type "Actor Object Reference") (OtherComp :type "PrimitiveComponent Object Reference") (OtherBodyIndex :type Integer) (bFromSweep :type Boolean) (SweepResult :type "HitResult Structure (by ref)"))
  (`/Engine/EditorBlueprintResources/ActorMacros.Switch Has Authority`
    (:`Authority`
      (bind _asutcharacter (cast `UTCharacter` OtherActor))
      (bind _astrials_player_controller (cast `TrialsPlayerController` (`Pawn.GetController` _asutcharacter)))
      (`TrialsPlayerController.SetCheckpoint` _astrials_player_controller self)
      (`/Engine/EditorBlueprintResources/StandardMacros.IsValid` (`TrialsPlayerController.CheckpointDest` _astrials_player_controller)
        (:`Is Valid`
          (`UTGameplayStatics.UTPlaySound` "/Engine/VREditor/Sounds/VR_teleport.VR_teleport" self "SRT_All" false (`self.K2_GetActorLocation` self) null _asutcharacter)
          (`GameplayStatics.SpawnEmitterAttached` (`self.SetEffect`) (`self.DefaultSceneRoot`))
          (`UTPlayerController.K2_ReceiveLocalizedMessage` _astrials_player_controller "/Trials/Blueprints/BP_Trials_Checkpoint_Message.BP_Trials_Checkpoint_Message_C" 0 null null null))))))

(fn `UserConstructionScript`
  (`self.K2_SetActorRotation` (`SceneComponent.K2_GetComponentRotation` (`self.Arrow`))))