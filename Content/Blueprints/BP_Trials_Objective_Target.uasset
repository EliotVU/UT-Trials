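; Trials objective target that completes its linked objective for the triggering player controller, on the server only.
; Shows an icon through a dynamic material instance built at construction, which GetScreenIcon also returns.
; Each cosmetic tick swaps the icon texture from the first player's objective state: inactive art when enabled but not active, active art otherwise, including when disabled.
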(event `self.ReceiveBeginPlay`
  (`/Engine/EditorBlueprintResources/StandardMacros.Can Execute Cosmetic Events`
    (:`True`
      (`SceneComponent.SetVisibility` (`self.Icon`) true false))))

(event `self.ReceiveTick`
  (params (DeltaSeconds :type "Float (single-precision)"))
  (bind _icon_instance (`self.Icon Instance`))
  (bind _objectiveinfo (`self.ObjectiveInfo`))
  (`/Engine/EditorBlueprintResources/StandardMacros.Can Execute Cosmetic Events`
    (:`True`
      (bind _asutplayer_controller (cast `UTPlayerController` (`GameplayStatics.GetPlayerController` 0)))
      (bind _returnvalue (`TrialsObjectiveInfo.IsEnabled` _objectiveinfo _asutplayer_controller))
      (if _returnvalue
        (bind _returnvalue_2 (`TrialsObjectiveInfo.IsActive` _objectiveinfo _asutplayer_controller))
        (if _returnvalue_2
          (`MaterialInstanceDynamic.SetTextureParameterValue` _icon_instance "Icon" (`self.Icon Active`) :!label _label)
          (else
            (`MaterialInstanceDynamic.SetTextureParameterValue` _icon_instance "Icon" (`self.Icon UnActive`))))
        (else
          (goto _label))))))

(event `Event Trigger`
  (params (Instigator :type "Controller Object Reference"))
  (`/Engine/EditorBlueprintResources/ActorMacros.Switch Has Authority`
    (:`Authority`
      (bind _asutplayer_controller (cast `UTPlayerController` Instigator))
      (`TrialsObjectiveInfo.CompleteObjective` (`self.ObjectiveInfo`) _asutplayer_controller))))

(fn `GetScreenIcon`
  (returns (ReturnValue :type "MaterialInterface Object Reference"))
  (bind _icon (`self.Icon`))
  (`/Engine/EditorBlueprintResources/StandardMacros.IsValid` _icon
    (:`Is Valid`
      (return (`PrimitiveComponent.GetMaterial` _icon 0)))
    (:`Is Not Valid`
      (return null))))

(fn `UserConstructionScript`
  (bind _returnvalue (`PrimitiveComponent.CreateDynamicMaterialInstance` (`self.Icon`) 0 null))
  (set `self.Icon Instance` _returnvalue))