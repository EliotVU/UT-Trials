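; BP_Trials_ShootTarget is a shootable target actor, apparently for trials, that reacts to incoming damage.
; AnyDamage runs a damage-type class check, then spawns the DamageImpact effect and a DamageEffect actor at the target's transform, passing the instigator to the impact effect.
; It then calls OnShot to signal the hit, and keeps no health or hit count of its own.
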(event `self.ReceiveAnyDamage`
  (params (Damage :type "Float (single-precision)") (DamageType :type "DamageType Object Reference") (InstigatedBy :type "Controller Object Reference") (DamageCauser :type "Actor Object Reference"))
  (if (`KismetMathLibrary.ClassIsChildOf` (`GameplayStatics.GetObjectClass` DamageType) (`self.Damage Type`))
    (`UTImpactEffect.CallSpawnEffect` self (`self.Damage Impact`) (`self.GetTransform` self) null self InstigatedBy)
    (`|SpawnActorFromClass` (`self.Damage Effect`) (`self.GetTransform` self) "AlwaysSpawn" "OverrideRootScale")
    (`self.On Shot`)))

(fn `UserConstructionScript`)